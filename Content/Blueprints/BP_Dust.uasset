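; Self-spreading dust cloud hazard that starts damage on the TopDownCharacter entering its large sphere and calls Heal on exit.
; On BeginPlay it removes itself without ground below, otherwise, if Spawn is set, starts a looping spawn timer, slower far from the player.
; Children appear at alternating diagonal offsets after random delays, limited by MaxChildren and the GameMode's OilMax.
; An inner sphere destroys overlapping clouds, fading the effect before removal.
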(event OnComponentBeginOverlap(SphereBig)
  (params (OverlappedComponent :type Primitive%20Component%20Object%20Reference) (OtherActor :type Actor%20Object%20Reference) (OtherComp :type Primitive%20Component%20Object%20Reference) (OtherBodyIndex :type Integer) (bFromSweep :type Boolean) (SweepResult :type Hit%20Result%20Structure%20%28by%20ref%29))
  ;[1 1 1] Урон по персонажу
  (bind _astop_down_character (Utilities|Casting|CastToTopDownCharacter OtherActor))
  (if (== (Variables|/Game/_CoreBP/TopDownCharacter.TopDownCharacter_C|GetCorallBody _astop_down_character) OtherComp)
    (Default|StartDamage _astop_down_character)))

(event OnComponentEndOverlap(SphereBig)
  (params (OverlappedComponent :type Primitive%20Component%20Object%20Reference) (OtherActor :type Actor%20Object%20Reference) (OtherComp :type Primitive%20Component%20Object%20Reference) (OtherBodyIndex :type Integer))
  ;[1 1 1] Урон по персонажу
  (bind _astop_down_character (Utilities|Casting|CastToTopDownCharacter OtherActor))
  (if (== (Variables|/Game/_CoreBP/TopDownCharacter.TopDownCharacter_C|GetCorallBody _astop_down_character) OtherComp)
    (Default|Heal _astop_down_character)))

(event OnComponentBeginOverlap(Sphere)
  (params (OverlappedComponent :type Primitive%20Component%20Object%20Reference) (OtherActor :type Actor%20Object%20Reference) (OtherComp :type Primitive%20Component%20Object%20Reference) (OtherBodyIndex :type Integer) (bFromSweep :type Boolean) (SweepResult :type Hit%20Result%20Structure%20%28by%20ref%29))
  ;[1 1 1] Чтобы на одном месте не было двух акторов сразу
  (bind _asbp_dust (Utilities|Casting|CastToBP_Dust OtherActor))
  (if (== (Variables|BP_Dust_C|GetSphere _asbp_dust) OtherComp)
    (CallFunction|Destroy _asbp_dust)))

(event Custom|Destroy
  ;[1 1 1] Уничтожение облака
  (Utilities|FlowControl|DoOnce false
    (:Completed
      (Components|Activation|Deactivate (Variables|Default|GetDust))
      (Utilities|FlowControl|Delay 1.0)
      (Actor|DestroyActor))))

(event Custom|SpawnDust
  (bind _rotated_ (Variables|Default|GetRotated?))
  ;[1 1 1] Алгоритм спавна
  (Utilities|CheckCount
    (:false
      (Utilities|FlowControl|Delay (Math|Random|RandomFloatinRange 0.0 (/ (Variables|Default|GetSpawnTime) 2.0)))
      (switch int (Math|Random|RandomIntegerinRange 0 1)
        (:0
          (if _rotated_
            (Variables|Default|SetLoc "-64.000000,64.000000, 0")
            (else
              (Variables|Default|SetLoc "64.000000,64.000000,0.000000"))))
        (:1
          (if _rotated_
            (Variables|Default|SetLoc "64.000000,-64.000000, 0")
            (else
              (Variables|Default|SetLoc "-64.000000,-64.000000, 0")))))
      (Game|SpawnActorfromClass "BP_Dust_C" (Math|Transform|MakeTransform (+ (Transformation|GetActorLocation) (Variables|Default|GetLoc)) (Math|Rotator|MakeRotator 0.0 0.0 (+ (.yaw (Transformation|GetActorRotation)) 9e+01)) "1,1,1") "AdjustIfPossibleButDontSpawnIfColliding" 0 true (not (Variables|Default|GetRotated?)) 0)
      (bind _result (Math|Integer|IncrementInt (Variables|Default|GetSpawned))
        (:%20%20
          (if (== _result (Variables|Default|GetMaxChildren))
            (Utilities|Time|ClearandInvalidateTimerbyHandle (Variables|Default|GetSpawnTimer))))))))

(event EventBeginPlay
  (bind _returnvalue (Transformation|GetActorLocation))
  ;[1 1 1] BeginPlay + SetTimer
  (bind _returnvalue_2 (Collision|LineTraceByChannel _returnvalue (- _returnvalue "0, 0,300.000000") "TraceTypeQuery3" false 0 "None" true "(R=1.000000,G=0.000000,B=0.000000,A=1.000000)" "(R=0.000000,G=1.000000,B=0.000000,A=1.000000)" 3.0))
  (if _returnvalue_2
    (if (Variables|Default|GetSpawn?)
      (if (< (Math|Vector|Distance(Vector) (Transformation|GetActorLocation) (Transformation|GetActorLocation (Game|Player|GetPlayerPawn 0))) (Variables|Default|GetDistanceTime))
        _
        (else
          (bind _output_get (Variables|Default|SetSpawnTime (* (Variables|Default|GetSpawnTime) 1.5)))))
      (bind _returnvalue_3 (Utilities|Time|SetTimerbyEvent (delegate Custom|SpawnDust) _output_get true))
      (Variables|Default|SetSpawnTimer _returnvalue_3))
    (else
      (CallFunction|Destroy))))

(fn ConstructionScript
  (bind _astop_down_game_mode (Utilities|Casting|CastToTopDownGameMode (Game|GetGameMode)))
  (Variables|Default|SetMax (Variables|/Game/_CoreBP/TopDownGameMode.TopDownGameMode_C|GetOilMax _astop_down_game_mode)))