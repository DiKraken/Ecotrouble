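; BP_Pipe is a pipe actor that periodically emits dust until it breaks.
; A looping timer, offset by a negative start delay to fire almost at once, replaces the previous BP_Dust with a new one above the pipe, randomly flagged as rotated.
; The Break event runs once, snapping the pipe to a fixed rotation and clearing the timer, without destroying the last dust actor.
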(event Custom|Break
  ;[1 1 1] Поломка трубы
  (Utilities|FlowControl|DoOnce false
    (:Completed
      (Transformation|SetWorldRotation (Variables|Default|GetPipe) "30.000000, 0,90.000000" false true)
      (Utilities|Time|ClearandInvalidateTimerbyHandle (Variables|Default|GetTimer)))))

(event Custom|Spawn
  (bind _returnvalue (Transformation|GetActorLocation))
  ;[1 1 1] Спавн частиц
  (Utilities|IsValid (Variables|Default|GetParticles)
    (:Is%20Valid
      (Actor|DestroyActor (Variables|Default|GetParticles)))
    (:Is%20Not%20Valid
      _))
  (bind _returnvalue_2 (Game|SpawnActorfromClass "/Game/Blueprints/BP_Dust.BP_Dust_C" (Math|Transform|MakeTransform (Math|Vector|MakeVector (.x _returnvalue) (.y _returnvalue) (+ (.z _returnvalue) 1.1e+02)) "0, 0, 0" "1,1,1") "Undefined" 0 true (Math|Random|RandomBool) 1 1 0))
  (Variables|Default|SetParticles _returnvalue_2))

(event EventBeginPlay
  (bind _time (Variables|Default|GetTime))
  (bind _returnvalue (Utilities|Time|SetTimerbyEvent (delegate Custom|Spawn) _time true (* _time -1.0)))
  (Variables|Default|SetTimer _returnvalue))

(fn ConstructionScript)