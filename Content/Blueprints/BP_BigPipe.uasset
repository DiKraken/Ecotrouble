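; Big pipe actor that periodically emits black dust until it is broken by damage.
; A looping timer, offset to fire at start, replaces the previous BP_BlackDust with a new, randomly rotated one above the pipe.
; Each Damage call tilts the pipe mesh and lowers HP, with a short DoOnce cooldown between hits.
; At zero HP, Destroy only clears the spawn timer, leaving the actor in place.
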(event Custom|Spawn
  (bind _returnvalue (Transformation|GetActorLocation))
  ;[1 1 1] Спавн частиц
  (Utilities|IsValid (Variables|Default|GetParticles)
    (:Is%20Valid
      (Actor|DestroyActor (Variables|Default|GetParticles)))
    (:Is%20Not%20Valid
      _))
  (bind _returnvalue_2 (Game|SpawnActorfromClass "/Game/Blueprints/BP_BlackDust.BP_BlackDust_C" (Math|Transform|MakeTransform (Math|Vector|MakeVector (.x _returnvalue) (.y _returnvalue) (+ (.z _returnvalue) 142.0)) "0, 0, 0" "1,1,1") "Undefined" 0 true (Math|Random|RandomBool) 3 0 0))
  (Variables|Default|SetParticles _returnvalue_2))

(event Custom|Damage
  (bind _pipe (Variables|Default|GetPipe))
  (bind _returnvalue (Transformation|GetWorldRotation _pipe))
  ;[1 1 1] Поломка трубы
  (Utilities|FlowControl|DoOnce false :!label _label
    (:Completed
      (Transformation|SetWorldRotation _pipe (Math|Rotator|MakeRotator (.roll _returnvalue) (+ (.pitch _returnvalue) 1e+01) (.yaw _returnvalue)) false true)
      (bind _result (Math|Integer|DecrementInt (Variables|Default|GetHP))
        (:%20%20
          (if (== _result 0)
            (CallFunction|Destroy)
            (else
              (Utilities|FlowControl|Delay 0.5)
              (goto _label Reset))))))))

(event Custom|Destroy
  ;[1 1 1] Поломка трубы
  (Utilities|FlowControl|DoOnce false
    (:Completed
      (Utilities|Time|ClearandInvalidateTimerbyHandle (Variables|Default|GetTimer)))))

(event EventBeginPlay
  (bind _time (Variables|Default|GetTime))
  (bind _returnvalue (Utilities|Time|SetTimerbyEvent (delegate Custom|Spawn) _time true (* _time -1.0)))
  (Variables|Default|SetTimer _returnvalue))

(fn ConstructionScript)